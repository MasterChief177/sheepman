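; Player character Blueprint that handles movement and mouse look input.
; Axis inputs feed movement along the actor's forward and right vectors, plus controller yaw and pitch.
; Sprint swaps max walk speed to a variable and restores a hard-coded default on release; crouch applies its own speed.
; Jump uses the built-in Character functions, with the jump height variable actually setting maximum hold time.
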(event Input|ActionEvents|InputActionJump
  (params (Key :type Key%20Structure :default "None"))
  ;[0.15 0.15 0.15 0.5] Movement System
  ;;[0.15 0.01554 0.02002 0.5] Jumping
  (:Pressed
    (Variables|Default|SetJumpMaxHoldTime (Variables|Default|GetJumpHeigt))
    (Character|Jump))
  (:Released
    (Character|StopJumping)))

(event Input|ActionEvents|InputActionCrouch
  (params (Key :type Key%20Structure :default "None"))
  ;[0.15 0.15 0.15 0.5] Movement System
  ;;[0.15 0.02029 0.02519 0.502] Crouch
  (:Pressed
    (Variables|/Script/Engine.CharacterMovementComponent|SetMaxWalkSpeedCrouched (Variables|Character|GetCharacterMovement) (Variables|Default|GetSpeenWhenCrouched))
    (Character|Crouch))
  (:Released
    (Character|UnCrouch)))

(event Input|ActionEvents|InputActionRun
  (params (Key :type Key%20Structure :default "None"))
  (bind _charactermovement (Variables|Character|GetCharacterMovement))
  ;[0.15 0.15 0.15 0.5] Movement System
  ;;[0.15 0.02029 0.02519 0.502] Running / Sprinting
  (:Pressed
    (Variables|/Script/Engine.CharacterMovementComponent|SetMaxWalkSpeed _charactermovement (Variables|Default|GetRunSpeed)))
  (:Released
    (Variables|/Script/Engine.CharacterMovementComponent|SetMaxWalkSpeed _charactermovement 6e+02)))

(event Input|AxisEvents|InputAxisForward_Backwars
  (params (AxisValue :type Float%20%28single-precision%29))
  ;[0.15 0.15 0.15 0.5] Movement System
  ;;[0.15 0.01392 0.01989 0.5] Forward and Backward
  (Pawn|Input|AddMovementInput (Transformation|GetActorForwardVector) AxisValue false))

(event Input|AxisEvents|InputAxisStrafe_Right_Left
  (params (AxisValue :type Float%20%28single-precision%29))
  ;[0.15 0.15 0.15 0.5] Movement System
  ;;[0.15 0.02029 0.02519 0.502] Strafing
  (Pawn|Input|AddMovementInput (Transformation|GetActorRightVector) AxisValue false))

(event Input|AxisEvents|InputAxisMouse_Rotate_Left_Right
  (params (AxisValue :type Float%20%28single-precision%29))
  ;[0.15 0.15 0.15 0.5] Look System
  (Pawn|Input|AddControllerYawInput AxisValue))

(event Input|AxisEvents|InputAxisMouse_Look_Up_Down
  (params (AxisValue :type Float%20%28single-precision%29))
  ;[0.15 0.15 0.15 0.5] Look System
  (Pawn|Input|AddControllerPitchInput AxisValue))

(fn ConstructionScript)